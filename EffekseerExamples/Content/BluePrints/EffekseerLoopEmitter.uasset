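; EffekseerLoopEmitter is an actor Blueprint that repeatedly plays an Effekseer particle effect while moving it.
; BeginPlay records the start location and plays the emitter, storing the handle.
; Each Tick moves the actor by Velocity, unscaled by delta time, and pushes position and rotation to the playing effect.
; When accumulated time exceeds Freq, the actor snaps back to its start and replays the effect.
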(event EventBeginPlay
  (bind _effekseeremitter (Variables|Default|GetEffekseerEmitter))
  (Utilities|FlowControl|Sequence
    (:then_0
      (Variables|Default|SetInitialLocation (Transformation|GetActorLocation (Components|GetOwner (Variables|Default|GetEffekseerEmitter)))))
    (:then_1
      (Transformation|SetActorLocation (Components|GetOwner _effekseeremitter) (Variables|Default|GetInitialLocation) false false)
      (bind _returnvalue (Class|EffekseerEmitterComponent|Play _effekseeremitter))
      (Variables|Default|SetPlayingHandle _returnvalue))))

(event EventActorBeginOverlap
  (params (OtherActor :type Actor%20Object%20Reference)))

(event EventTick
  (params (DeltaSeconds :type Float%20%28single-precision%29))
  (bind _effekseeremitter (Variables|Default|GetEffekseerEmitter))
  (bind _effekseeremitter_2 (Variables|Default|GetEffekseerEmitter))
  (bind _velocity (Variables|Default|GetVelocity))
  (bind _returnvalue (Components|GetOwner _effekseeremitter))
  (bind _returnvalue_2 (Transformation|GetActorLocation _returnvalue))
  (bind _returnvalue_3 (+ _returnvalue_2 _velocity))
  (Utilities|FlowControl|Sequence
    (:then_0
      (Transformation|SetActorLocation _returnvalue _returnvalue_3 false false)
      (Class|EffekseerSystemComponent|SetEffectPosition (Utilities|Struct|BreakEffekseerHandle (Variables|Default|GetPlayingHandle)) (Variables|Default|GetPlayingHandle) _returnvalue_3)
      (Class|EffekseerSystemComponent|SetEffectRotation (Utilities|Struct|BreakEffekseerHandle (Variables|Default|GetPlayingHandle)) (Variables|Default|GetPlayingHandle) (Transformation|GetActorRotation _returnvalue)))
    (:then_1
      (Variables|Default|SetTime (+ DeltaSeconds (Variables|Default|GetTime))))
    (:then_2
      (if (> (Variables|Default|GetTime) (Variables|Default|GetFreq))
        (Variables|Default|SetTime 0.0)
        (Transformation|SetActorLocation (Components|GetOwner _effekseeremitter_2) (Variables|Default|GetInitialLocation) false false)
        (bind _returnvalue_4 (Class|EffekseerEmitterComponent|Play _effekseeremitter_2))
        (Variables|Default|SetPlayingHandle _returnvalue_4)))))

(fn ConstructionScript)